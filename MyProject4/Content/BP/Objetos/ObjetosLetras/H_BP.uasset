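; H_BP is a collectible letter object for the letter H, picked up when the level 1 player character (PJ_level1) overlaps its HidBox.
; On overlap it adds "H" to the GameInstance's ListaEncont1 found list and refreshes the player's word HUD through PalabraPantalla.
; It then opens a WidgetP question widget, destroys itself and switches input to UI only.
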(event `self.hidBox.OnComponentBeginOverlap`
  (params (OverlappedComponent :type "PrimitiveComponent Object Reference") (OtherActor :type "Actor Object Reference") (OtherComp :type "PrimitiveComponent Object Reference") (OtherBodyIndex :type Integer) (bFromSweep :type Boolean) (SweepResult :type "HitResult Structure (by ref)"))
  (bind _aspj_level_1 (cast `/Game/BP/PJ_level1` OtherActor))
  (bind _asgameinstance_p (cast `/Game/BP/GameinstanceP` (`GameplayStatics.GetGameInstance`)))
  (`KismetArrayLibrary.Array_AddUnique` (`/Game/BP/GameinstanceP.ListaEncont_1` _asgameinstance_p) "H")
  (`/Game/UI/PalabrasHUD.PalabraPantalla` (`/Game/BP/PJ_level1.PalabrasHUD` _aspj_level_1))
  (bind _returnvalue (`|CreateWidget` "/Game/UI/WidgetP.WidgetP_C"))
  (bind _output_get (set `self.PreguntaWidget` _returnvalue))
  (`UserWidget.AddToViewport` _output_get 0)
  (`self.K2_DestroyActor`)
  (`/Engine/EditorBlueprintResources/StandardMacros.IsValid` null
    (:`Is Valid`
      _)
    (:`Is Not Valid`
      _))
  (`WidgetBlueprintLibrary.SetInputMode_UIOnlyEx` (`GameplayStatics.GetPlayerController` 0) null))

(fn `UserConstructionScript`)